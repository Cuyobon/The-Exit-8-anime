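; Spline-following NPC that moves its InjuredWalking component along the actor's spline at WalkSpeed.
; Each Tick advances the stored distance by frame time, then applies that point's local-space location and rotation to the component, keeping its scale.
; Fixed height and yaw offsets correct the component's placement and facing.
; Distance has no wrap or clamp in the graph; the ResetSplinePos event returns it to the start.
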(event `self.ReceiveTick`
  (params (DeltaSeconds :type "Float (single-precision)"))
  (bind _returnvalue (`SplineComponent.GetTransformAtDistanceAlongSpline` (`self.Spline`) (`self.DistanceAlongTheSpline`) "Local" false))
  (set `self.DistanceAlongTheSpline` (+ (* DeltaSeconds (`self.WalkSpeed`)) (`self.DistanceAlongTheSpline`)))
  (`SceneComponent.K2_SetRelativeTransform` (`self.Injured_Walking`) (`KismetMathLibrary.MakeTransform` (`KismetMathLibrary.MakeVector` (.x (.location _returnvalue)) (.y (.location _returnvalue)) (+ (.z (.location _returnvalue)) -90.0)) (`KismetMathLibrary.MakeRotator` (.roll (.rotation _returnvalue)) (.pitch (.rotation _returnvalue)) (+ (.yaw (.rotation _returnvalue)) -90.0)) (`SceneComponent.RelativeScale3D` (`self.Injured_Walking`))) false false))

(event `ResetSplinePos`
  (set `self.DistanceAlongTheSpline` 0.0))

(fn `UserConstructionScript`)